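; BP_King is the King blueprint, providing entry points for spawning four soldier types or slots by index.
; Spawn01 to Spawn04 each pass a fixed zero-based index to SpawnSoldierByIndex.
; ForLoopSpawn01 to ForLoopSpawn04 do the same through ForloopSpawnSoldierByIndex.
; The spawn logic is not defined in these graphs, and BeginPlay, overlap, Tick and the construction script are empty.
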(event Custom|ForLoopSpawn04
  (Class|SandBoxPeopleKing|ForloopSpawnSoldierbyIndex 3))

(event Custom|Spawn01
  (Class|SandBoxPeopleKing|SpawnSoldierbyIndex))

(event Custom|ForLoopSpawn03
  (Class|SandBoxPeopleKing|ForloopSpawnSoldierbyIndex 2))

(event Custom|Spawn04
  (Class|SandBoxPeopleKing|SpawnSoldierbyIndex 3))

(event Custom|Spawn02
  (Class|SandBoxPeopleKing|SpawnSoldierbyIndex 1))

(event Custom|Spawn03
  (Class|SandBoxPeopleKing|SpawnSoldierbyIndex 2))

(event Custom|ForLoopSpawn01
  (Class|SandBoxPeopleKing|ForloopSpawnSoldierbyIndex))

(event Custom|ForLoopSpawn02
  (Class|SandBoxPeopleKing|ForloopSpawnSoldierbyIndex 1))

(event EventBeginPlay)

(event Collision|EventActorBeginOverlap
  (params (OtherActor :type Actor%20Object%20Reference)))

(event EventTick
  (params (DeltaSeconds :type Float%20%28single-precision%29)))

(fn ConstructionScript)