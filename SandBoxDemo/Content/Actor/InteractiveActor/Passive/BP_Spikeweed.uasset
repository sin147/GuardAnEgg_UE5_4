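; Spikeweed trap, a passive interactive actor that raises thorns and periodically damages characters standing over them.
; The pre-interact and break phases slide the Thron component up and back down based on state progress.
; While interacting, a timer box-traces the Pawn profile each second, with debug drawing, and damages each SandBoxCharacter hit through the damage subsystem.
; The interaction-start trace currently does nothing, as its damage call is unconnected.
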(event EventBeginPlay
  (|CallParentFunction) ; This node is disabled and will not be called.\nDrag off pins to build functionality.
)

(event Collision|EventActorBeginOverlap
  (params (OtherActor :type Actor%20Object%20Reference))
  (|CallParentFunction OtherActor) ; This node is disabled and will not be called.\nDrag off pins to build functionality.
)

(event EventTick
  (params (DeltaSeconds :type Float%20%28single-precision%29))
  (|CallParentFunction DeltaSeconds) ; This node is disabled and will not be called.\nDrag off pins to build functionality.
)

(event EventPreInteractImp
  (params (InCurrentlyStateTime :type Float%20%28single-precision%29) (InTotalDurationTime :type Float%20%28single-precision%29) (InDeltaTime :type Float%20%28single-precision%29))
  (Transformation|SetRelativeLocation (Variables|Default|GetThron) (Math|Vector|MakeVector 0.0 0.0 (* (- 1.0 (/ InCurrentlyStateTime InTotalDurationTime)) -6e+01)) false false))

(event EventInteractBreakImp
  (params (InCurrentlyStateTime :type Float%20%28single-precision%29) (InTotalDurationTime :type Float%20%28single-precision%29) (InDeltaTime :type Float%20%28single-precision%29))
  (Transformation|SetRelativeLocation (Variables|Default|GetThron) (Math|Vector|MakeVector 0.0 0.0 (* (/ InCurrentlyStateTime InTotalDurationTime) -6e+01)) false false))

(event EventInteracttingImp
  (params (InCurrentlyStateTime :type Float%20%28single-precision%29) (InTotalDurationTime :type Float%20%28single-precision%29) (InDeltaTime :type Float%20%28single-precision%29))
  (bind _thron (Variables|Default|GetThron))
  (bind _returnvalue (Transformation|GetWorldLocation _thron))
  (bind _returnvalue_2 (+ (.z _returnvalue) 3e+01))
  (bind _output_get (Variables|Default|SetInteracttingTime (+ InDeltaTime (Variables|Default|GetInteracttingTime))))
  (if (>= _output_get 1.0)
    (Variables|Default|SetInteracttingTime 0.0)
    (bind _outhits (Class|KismetSystemLibrary|BoxTraceMultibyProfile (Math|Vector|MakeVector (.x _returnvalue) (.y _returnvalue) _returnvalue_2) (Math|Vector|MakeVector (.x _returnvalue) (.y _returnvalue) _returnvalue_2) "140.000000,140.000000,30.000000" "0, 0, 0" "Pawn" false 0 "ForDuration" true "(R=1.000000,G=0.000000,B=0.000000,A=1.000000)" "(R=0.000000,G=1.000000,B=0.000000,A=1.000000)" 1.0))
    (for _array_element _outhits
      (bind _assand_box_character (Utilities|Casting|CastToSandBoxCharacter (.hitactor _array_element)))
      (Class|DamageSubsytem|TakeDamage (Subsystems|GetDamageSubsytem) _assand_box_character 1e+01 self))))

(event EventStartInteractImp
  (params (InCurrentlyStateTime :type Float%20%28single-precision%29) (InTotalDurationTime :type Float%20%28single-precision%29) (InDeltaTime :type Float%20%28single-precision%29))
  (bind _thron (Variables|Default|GetThron))
  (bind _returnvalue (Transformation|GetWorldLocation _thron))
  (bind _returnvalue_2 (+ (.z _returnvalue) 3e+01))
  (bind _outhits (Class|KismetSystemLibrary|BoxTraceMulti (Math|Vector|MakeVector (.x _returnvalue) (.y _returnvalue) _returnvalue_2) (Math|Vector|MakeVector (.x _returnvalue) (.y _returnvalue) _returnvalue_2) "140.000000,140.000000,30.000000" "0, 0, 0" "TraceTypeQuery1" false 0 "ForOneFrame" true "(R=1.000000,G=0.000000,B=0.000000,A=1.000000)" "(R=0.000000,G=1.000000,B=0.000000,A=1.000000)" 1.0))
  (for _array_element _outhits
    _))

(fn ConstructionScript
  (|CallParentFunction))